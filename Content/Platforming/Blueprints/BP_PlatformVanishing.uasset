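; A platforming platform that vanishes once the player has stood on it for its set lifetime, then reappears.
; Trigger zone overlaps flag the player's presence, and Tick accumulates time while the flag is set, resetting it otherwise.
; At the limit it hides and disables collision, waits, then restores the transform saved at BeginPlay, visibility and collision.
; Debug strings print overlap changes and the running timer.
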(event OnComponentBeginOverlap(PlatformTriggerzone)
  (params (OverlappedComponent :type Primitive%20Component%20Object%20Reference) (OtherActor :type Actor%20Object%20Reference) (OtherComp :type Primitive%20Component%20Object%20Reference) (OtherBodyIndex :type Integer) (bFromSweep :type Boolean) (SweepResult :type Hit%20Result%20Structure%20%28by%20ref%29))
  ;[0.3557 0.6299 1] Colider Check
  (if (== OtherActor (Game|Player|GetPlayerPawn 0))
    (Utilities|FlowControl|Sequence
      (:then_0
        (Development|PrintString "IDK u tell me ARE you on the platform?"))
      (:then_1
        (Variables|Default|SetIsPlayerOnPlatform true)))))

(event OnComponentEndOverlap(PlatformTriggerzone)
  (params (OverlappedComponent :type Primitive%20Component%20Object%20Reference) (OtherActor :type Actor%20Object%20Reference) (OtherComp :type Primitive%20Component%20Object%20Reference) (OtherBodyIndex :type Integer))
  ;[0.3557 0.6299 1] Colider Check
  (if (== OtherActor (Game|Player|GetPlayerPawn 0))
    (Utilities|FlowControl|Sequence
      (:then_0
        (Development|PrintString "L no platform"))
      (:then_1
        (Variables|Default|SetIsPlayerOnPlatform false)))))

(event Custom|ReturnToStart
  ;[1 0.756 0.1085] Return to start
  (Transformation|SetWorldTransform (Variables|Default|GetDefaultSceneRoot) (Math|Transform|MakeTransform (Variables|Default|GetStartLocation) (Variables|Default|GetStartRotation) (Variables|Default|GetStartScale)) false true)
  (Variables|Default|SetTimeOnPlatform 0.0)
  (Rendering|SetActorHiddenInGame false)
  (Collision|SetActorEnableCollision true))

(event EventBeginPlay
  (bind _returnvalue (Transformation|GetActorTransform))
  ;[1 0.6042 0.9067] Set Strating Variables
  (Variables|Default|SetStartLocation (.location _returnvalue))
  (Variables|Default|SetStartRotation (.rotation _returnvalue))
  (Variables|Default|SetStartScale (.scale _returnvalue)))

(event EventTick
  (params (DeltaSeconds :type Float%20%28single-precision%29))
  ;[0.4407 1 0.3501] Platform Timer
  (if (Variables|Default|GetIsPlayerOnPlatform)
    (bind _output_get (Variables|Default|SetTimeOnPlatform (+ (Variables|Default|GetTimeOnPlatform) DeltaSeconds)))
    (Utilities|FlowControl|Sequence
      (:then_0
        ;[1 0.6695 0.6095] Timer check >= platform lifetime
        (if (>= (Variables|Default|GetTimeOnPlatform) (Variables|Default|GetPlatformLifetime))
          ;[0.9889 0.4172 1] Platform Collision
          (Rendering|SetActorHiddenInGame true)
          (Collision|SetActorEnableCollision false)
          (Utilities|FlowControl|Delay (Variables|Default|GetTimeInvisible))
          (CallFunction|ReturntoStart)))
      (:then_1
        (Development|PrintString (Utilities|String|ToString(Float) _output_get))))
    (else
      (Variables|Default|SetTimeOnPlatform 0.0))))

(fn ConstructionScript)
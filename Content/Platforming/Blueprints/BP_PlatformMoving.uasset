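; BP_PlatformMoving is a platforming actor that moves back and forth along a straight line.
; On BeginPlay it enables movement and starts a looping timer that reverses its Direction vector every MovementDuration seconds.
; Each Tick offsets the actor by the normalized Direction times Speed, without sweep or delta-time scaling, so its speed depends on frame rate.
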(event Custom|FlipDirection
  ;[0.5398 0.3401 1] Platform Flip Direction
  (Variables|Default|SetDirection (* (Variables|Default|GetDirection) -1.0)))

(event EventTick
  (params (DeltaSeconds :type Float%20%28single-precision%29))
  ;[0.3281 0.006836 0.006836] Platform Movement
  (if (Variables|Default|GetCanPlatformMove)
    (Transformation|AddActorWorldOffset (* (Math|Vector|Normalize (Variables|Default|GetDirection)) (Variables|Default|GetSpeed)))))

(event EventBeginPlay
  ;[0.5398 0.3401 1] Platform Flip Direction
  (Utilities|FlowControl|Sequence
    (:then_0
      (Variables|Default|SetCanPlatformMove true))
    (:then_1
      (Utilities|Time|SetTimerbyEvent (delegate Custom|FlipDirection) (Variables|Default|GetMovementDuration) true))))

(fn ConstructionScript)
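; BP_Enemy_Turret is an enemy turret that continuously fires BP_Bullet actors from its FiringPoint.
; Each Tick, if LookAtPlayer is set, it rotates SMStem using a look-at rotation computed from X/Y positions toward the player pawn.
; BeginPlay uses UseScatterShot to choose single shots or bursts with random yaw spread.
; Each firing event re-calls itself after FiringDelay, forming an endless loop.
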(event Custom|One%20Shot
  ;[1 0.5528 0] One shot
  (Game|SpawnActorfromClass "/Game/Platforming/Blueprints/BP_Bullet.BP_Bullet_C" (Transformation|GetSocketTransform (Variables|Default|GetFiringPoint) "None" "RTS_World") "Undefined" "MultiplyWithRoot" 0 0)
  ;[0.116 1 0.6843] Re-Call one shot
  (Utilities|FlowControl|Delay (Variables|Default|GetFiringDelay))
  (CallFunction|OneShot))

(event Custom|Scatter%20Shot
  (bind _firingpoint (Variables|Default|GetFiringPoint))
  (bind _returnvalue (Transformation|GetSocketTransform _firingpoint "None" "RTS_World"))
  ;[1 0.3991 0.7365] Scatter shot
  (for _index (range 0 5)
    (Game|SpawnActorfromClass "/Game/Platforming/Blueprints/BP_Bullet.BP_Bullet_C" (Math|Transform|MakeTransform (.location _returnvalue) (Math|Rotator|MakeRotator (.roll (.rotation _returnvalue)) (.pitch (.rotation _returnvalue)) (+ (.yaw (.rotation _returnvalue)) (Math|Random|RandomFloatinRange -3e+01 3e+01)))) "Undefined" "MultiplyWithRoot" 0 0))
  ;[0.5297 1 0.3197] Re-call scatter shot
  (Utilities|FlowControl|Delay (Variables|Default|GetFiringDelay))
  (CallFunction|ScatterShot))

(event EventBeginPlay
  ;[0.06894 0.05872 0.15 0.5] Set up firing shot
  (if (Variables|Default|GetUseScatterShot)
    (CallFunction|ScatterShot)
    (else
      (CallFunction|OneShot))))

(event EventTick
  (params (DeltaSeconds :type Float%20%28single-precision%29))
  (bind _returnvalue (Game|Player|GetPlayerPawn 0))
  (bind _returnvalue_2 (Transformation|GetActorLocation))
  (bind _returnvalue_3 (Transformation|GetActorLocation _returnvalue))
  ;[0.3469 0.2222 1] Look at player
  (if (Variables|Default|GetLookAtPlayer)
    (Transformation|SetRelativeRotation (Variables|Default|GetSM_Stem) (Math|Rotator|FindLookatRotation (Math|Vector|MakeVector (.x _returnvalue_2) (.y _returnvalue_2) 0.0) (Math|Vector|MakeVector (.x _returnvalue_3) (.y _returnvalue_3) 0.0)) false false)))

(fn ConstructionScript)
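; BP_Bullet is a projectile actor that damages the player's third-person character on contact.
; Each Tick it moves along its normalized local Direction by Speed, without sweeping or delta-time scaling, and a Delay started from Tick destroys it after BulletLifetime.
; An overlap on SM_Bullet with the player cached at BeginPlay calls DamagePlayer, then destroys the bullet after a short delay.
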(event OnComponentBeginOverlap(SM_Bullet)
  (params (OverlappedComponent :type Primitive%20Component%20Object%20Reference) (OtherActor :type Actor%20Object%20Reference) (OtherComp :type Primitive%20Component%20Object%20Reference) (OtherBodyIndex :type Integer) (bFromSweep :type Boolean) (SweepResult :type Hit%20Result%20Structure%20%28by%20ref%29))
  ;[0.8943 0 1] Player Damage
  (if (== OtherActor (Variables|Default|GetPlayer%20Reference))
    (Default|DamagePlayer (Variables|Default|GetPlayer%20Reference) (Variables|Default|GetDamage))
    (Utilities|FlowControl|Delay 0.2)
    ;[1 0.28 0] Destroy Bullet
    (Actor|DestroyActor)))

(event EventBeginPlay
  ;[0.1667 0.6998 1] Get Player Reference
  (bind _asbp_third_person_character (Utilities|Casting|CastToBP_ThirdPersonCharacter (Game|Player|GetPlayerPawn 0)))
  (Variables|Default|SetPlayer%20Reference _asbp_third_person_character))

(event EventTick
  (params (DeltaSeconds :type Float%20%28single-precision%29))
  ;[0.2249 1 0] Bullet Movement
  (Transformation|AddActorLocalOffset (* (Math|Vector|Normalize (Variables|Default|GetDirection)) (Variables|Default|GetSpeed)) false false)
  ;[1 0 0.03895] Destroy Bullet
  (Utilities|FlowControl|Delay (Variables|Default|GetBulletLifetime))
  (Actor|DestroyActor))

(fn ConstructionScript)
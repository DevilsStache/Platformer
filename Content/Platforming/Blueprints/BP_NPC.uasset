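; BP_NPC is a talkable NPC that shows an interaction prompt widget while the player is inside its trigger zone.
; On BeginPlay it caches the player's third-person character.
; ResetDialogue restarts the dialogue, and UpdateDialogue writes each line into the character's CurrentDialogueText on a timed delay, calling itself until the lines run out, then clearing the text.
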(event OnComponentBeginOverlap(NPCTriggerZone)
  (params (OverlappedComponent :type Primitive%20Component%20Object%20Reference) (OtherActor :type Actor%20Object%20Reference) (OtherComp :type Primitive%20Component%20Object%20Reference) (OtherBodyIndex :type Integer) (bFromSweep :type Boolean) (SweepResult :type Hit%20Result%20Structure%20%28by%20ref%29))
  ;[0.15 0.02309 0.06124 0.5] Player Checks
  (if (Actor|ActorHasTag OtherActor "Player")
    (Rendering|SetVisibility (Variables|Default|GetW_InteractionPrompt) true false)))

(event OnComponentEndOverlap(NPCTriggerZone)
  (params (OverlappedComponent :type Primitive%20Component%20Object%20Reference) (OtherActor :type Actor%20Object%20Reference) (OtherComp :type Primitive%20Component%20Object%20Reference) (OtherBodyIndex :type Integer))
  ;[0.15 0.02309 0.06124 0.5] Player Checks
  (if (Actor|ActorHasTag OtherActor "Player")
    (Rendering|SetVisibility (Variables|Default|GetW_InteractionPrompt) false false)))

(event Custom|UpdateDialogue
  ;[0 0.9635 0.738 0.5] Update Dialogue
  (Variables|/Game/Platforming/Blueprints/BP_ThirdPersonCharacter.BP_ThirdPersonCharacter_C|SetCurrentDialogueText (Variables|Default|GetPlayer%20Reference) (Utilities|Array|Get(acopy) (Variables|Default|GetDialogueLine) (Variables|Default|GetCurrentDialogueLine)))
  (Variables|Default|SetCurrentDialogueLine (+ (Variables|Default|GetCurrentDialogueLine) 1))
  (Utilities|FlowControl|Delay 2.0)
  (if (!= (Variables|Default|GetCurrentDialogueLine) (Utilities|Array|Length (Variables|Default|GetDialogueLine)))
    (CallFunction|UpdateDialogue)
    (else
      (Variables|/Game/Platforming/Blueprints/BP_ThirdPersonCharacter.BP_ThirdPersonCharacter_C|SetCurrentDialogueText (Variables|Default|GetPlayer%20Reference) ""))))

(event Custom|ResetDialogue
  ;[0.15 0.0543 0.1478 0.5] Reset Dialogue
  (Variables|Default|SetCurrentDialogueLine 0)
  (CallFunction|UpdateDialogue))

(event EventBeginPlay
  (bind _asbp_third_person_character (Utilities|Casting|CastToBP_ThirdPersonCharacter (Game|Player|GetPlayerPawn 0)))
  (Variables|Default|SetPlayer%20Reference _asbp_third_person_character))

(fn ConstructionScript)
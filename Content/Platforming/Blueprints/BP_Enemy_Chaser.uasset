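; Platforming enemy that faces and chases the player once they enter its detection range; only a non-player actor leaving that range clears detection.
; Overlapping the HitZone bounces the player and removes health, while capsule hits knock the player back along the enemy's velocity and deal damage.
; At zero health, a random-count loop spawns coins at world origin, not the enemy's location, and calls DestroyActor inside the loop.
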(event OnComponentBeginOverlap(Detection_Range)
  (params (OverlappedComponent :type Primitive%20Component%20Object%20Reference) (OtherActor :type Actor%20Object%20Reference) (OtherComp :type Primitive%20Component%20Object%20Reference) (OtherBodyIndex :type Integer) (bFromSweep :type Boolean) (SweepResult :type Hit%20Result%20Structure%20%28by%20ref%29))
  ;[0.5839 0.3474 1] Check if detecting player
  (if (== OtherActor (Variables|Default|GetPlayerReference))
    (Variables|Default|SetCanDetectPlayer true)))

(event OnComponentEndOverlap(Detection_Range)
  (params (OverlappedComponent :type Primitive%20Component%20Object%20Reference) (OtherActor :type Actor%20Object%20Reference) (OtherComp :type Primitive%20Component%20Object%20Reference) (OtherBodyIndex :type Integer))
  ;[0.5839 0.3474 1] Check if detecting player
  (if (not (== OtherActor (Variables|Default|GetPlayerReference)))
    (Variables|Default|SetCanDetectPlayer false)))

(event OnComponentBeginOverlap(HitZone)
  (params (OverlappedComponent :type Primitive%20Component%20Object%20Reference) (OtherActor :type Actor%20Object%20Reference) (OtherComp :type Primitive%20Component%20Object%20Reference) (OtherBodyIndex :type Integer) (bFromSweep :type Boolean) (SweepResult :type Hit%20Result%20Structure%20%28by%20ref%29))
  ;[0.03127 0 1] Enemy head bounce
  (if (== OtherActor (Variables|Default|GetPlayerReference))
    (Utilities|FlowControl|Sequence
      (:then_0
        ;[1 0.3642 0.3841] launch character off enemy head
        (Character|LaunchCharacter (Variables|Default|GetPlayerReference) (Variables|Default|GetLaunchDirection) false false))
      (:then_1
        ;[0.8916 0.2746 1] Calculate enemy health
        (Variables|Default|SetHealth (- (Variables|Default|GetHealth) 1))
        ;[0.3411 1 0.4424] Destroy enemy
        (if (<= (Variables|Default|GetHealth) 0)
          (CallFunction|LootandDestroy))))))

(event OnComponentHit(CapsuleComponent)
  (params (HitComponent :type Primitive%20Component%20Object%20Reference) (OtherActor :type Actor%20Object%20Reference) (OtherComp :type Primitive%20Component%20Object%20Reference) (NormalImpulse :type Vector :default "0, 0, 0") (Hit :type Hit%20Result%20Structure%20%28by%20ref%29))
  ;[0.4892 1 0.8273] Player Knockback
  (if (== OtherActor (Variables|Default|GetPlayerReference))
    (Character|LaunchCharacter (Variables|Default|GetPlayerReference) (* (Transformation|GetVelocity) (Variables|Default|GetKnockbackStrength)) false false)
    ;[0.03885 0.04672 0.15 0.5] Damage Player
    (Default|DamagePlayer (Variables|Default|GetPlayerReference) (Variables|Default|GetDamage))))

(event Custom|LootAndDestroy
  (bind _returnvalue (Transformation|GetActorTransform))
  ;[0.1306 0.02324 0.15 0.5] Coin Drop On Death
  (for _index (range 0 (Math|Random|RandomIntegerinRange 0 9))
    (Game|SpawnActorfromClass "/Game/Platforming/Blueprints/BP_Coin.BP_Coin_C" (Math|Transform|MakeTransform "0, 0, 0" (.rotation _returnvalue) (.scale _returnvalue)) "Undefined" "MultiplyWithRoot" 0 0)
    (Actor|DestroyActor)))

(event EventBeginPlay
  ;[1 0.3228 0.3328] Get Player Reference
  (bind _asbp_third_person_character (Utilities|Casting|CastToBP_ThirdPersonCharacter (Game|Player|GetPlayerPawn 0)))
  (Variables|Default|SetPlayerReference _asbp_third_person_character))

(event EventTick
  (params (DeltaSeconds :type Float%20%28single-precision%29))
  (bind _returnvalue (Transformation|GetActorLocation))
  (bind _playerreference (Variables|Default|GetPlayerReference))
  (bind _returnvalue_2 (Transformation|GetActorLocation _playerreference))
  ;[0.3521 1 0.1896] If player detected
  (if (Variables|Default|GetCanDetectPlayer)
    (Utilities|FlowControl|Sequence
      (:then_0
        ;[0.4794 1 0.8275] Look at player
        (Transformation|SetActorRotation (Math|Rotator|FindLookatRotation (Math|Vector|MakeVector (.x _returnvalue) (.y _returnvalue) 0.0) (Math|Vector|MakeVector (.x _returnvalue_2) (.y _returnvalue_2) 0.0))))
      (:then_1
        ;[1 0.7928 0.2557] Chase Player
        (Pawn|Input|AddMovementInput (Math|Vector|Normalize (- (Transformation|GetActorLocation (Variables|Default|GetPlayerReference)) (Transformation|GetActorLocation))) 1.0 false)))))

(fn ConstructionScript)